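; BP_Balloon is a randomly colored helium balloon that reports to the PAZ game mode when destroyed.
; Construction randomizes a dynamic material's base color and the Mass variable, which varies buoyancy between balloons.
; Tick applies buoyancy minus weight, from air and helium densities, volume and gravity, to the capsule as a vertical acceleration-change force.
; BeginPlay binds OnDestroyed to OnBalloonPop, which calls GM_PAZ's OnBalloonPopped.
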(event `self.ReceiveTick`
  (params (DeltaSeconds :type "Float (single-precision)"))
  (bind _gravity (`self.Gravity`))
  ;[1 1 1] Physics
  (`PrimitiveComponent.AddForce` (`self.Capsule`) (`KismetMathLibrary.MakeVector` 0.0 0.0 (- (* (- (`self.Air Density`) (`self.Helium Density`)) (`self.Volume`) _gravity) (* _gravity (`self.Mass`)))) "None" true))

(event `self.ReceiveBeginPlay`
  (add `self.OnDestroyed` (delegate `OnBalloonPop`)))

(event `OnBalloonPop`
  ;[1 1 1] Send a message to the gamemode to indicate a balloon is destroyed
  (bind _asgm_paz (cast `/Game/PAZ/Blueprint/GM_PAZ` (`GameplayStatics.GetGameMode`)))
  (`/Game/PAZ/Blueprint/GM_PAZ.OnBalloonPopped` _asgm_paz))

(fn `UserConstructionScript`
  ;[1 1 1] Randomly assign a color for the balloon
  (bind _returnvalue (`PrimitiveComponent.CreateDynamicMaterialInstance` (`self.Balloon`) 0 "/Game/PAZ/Material/Mat_Balloon.Mat_Balloon"))
  (`MaterialInstanceDynamic.SetVectorParameterValue` _returnvalue "Base Color" (make `LinearColor` (`KismetMathLibrary.RandomFloatInRange` 0.0 1.0) (`KismetMathLibrary.RandomFloatInRange` 0.0 1.0) (`KismetMathLibrary.RandomFloatInRange` 0.0 1.0) 1.0))
  ;[1 1 1] Give the balloon a random mass as pseudo-control over bouyancy
  (set `self.Mass` (`KismetMathLibrary.RandomFloatInRange` 0.003 0.1)))