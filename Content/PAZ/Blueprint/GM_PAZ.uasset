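; Game mode for a first-person balloon-shooting game, running the menu, levels and win/lose checks.
; BeginPlay creates title, goal and HUD widgets, binds a tagged HUD trigger, fills the level array and spawns the first level's balloons.
; While the player is disabled, input drives the menus, tracked through one active-widget reference.
; After each shot, a delayed remaining-balloon count completes the level or ends the game, as does timeout.
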(event `self.ReceiveBeginPlay`
  (bind _returnvalue (`GameplayStatics.GetPlayerController` 0))
  (bind _levels (`self.Levels`))
  (`|ExecutionSequence`
    (:`then_0`
      ;[1 1 1] Enable the gamemode to receive input from the player, and disable movement/shooting at the start
      (`self.EnableInput` _returnvalue)
      (bind _asfirst_person_character (cast `/Game/FirstPersonBP/Blueprints/FirstPersonCharacter` (`GameplayStatics.GetPlayerCharacter` 0)))
      (`/Game/FirstPersonBP/Blueprints/FirstPersonCharacter.DIsableFPSPlayer` _asfirst_person_character))
    (:`then_1`
      ;[1 1 1] Add HUD widgets to the scene
      (bind _returnvalue_2 (`|CreateWidget` "/Game/PAZ/Widgets/TitleScreen.TitleScreen_C" _returnvalue))
      (bind _output_get (set `self.TitleScreenInstance` _returnvalue_2))
      (`UserWidget.AddToViewport` _output_get 0)
      (set `self.ActiveWidget` _output_get))
    (:`then_2`
      (bind _returnvalue_3 (`|CreateWidget` "/Game/PAZ/Widgets/GoalScreen.GoalScreen_C" _returnvalue))
      (bind _output_get_2 (set `self.GoalScreenInstance` _returnvalue_3))
      (`UserWidget.AddToViewport` _output_get_2 0)
      (`Widget.SetVisibility` _output_get_2 "Hidden"))
    (:`then_3`
      (bind _returnvalue_4 (`|CreateWidget` "/Game/PAZ/Widgets/HUD.HUD_C"))
      (bind _output_get_3 (set `self.HUDWidgetInstance` _returnvalue_4))
      (`UserWidget.AddToViewport` _output_get_3 0)
      (`Widget.SetVisibility` _output_get_3 "Hidden"))
    (:`then_4`
      ;[1 1 1] Find tagged trigger volume and store a reference to it
      (bind _outactors (`GameplayStatics.GetAllActorsOfClass` "/Script/Engine.TriggerVolume"))
      (for _array_element _outactors
        (if (`self.ActorHasTag` _array_element "HUDTrigger")
          (break)))
      (bind _output_get_4 (set `self.HUDTriggerVolume` _array_element))
      ;[1 1 1] Bind the trigger's overlaps to custom events
      (add `self.OnActorBeginOverlap` _output_get_4 (delegate `OnHUDTriggerEnter`))
      (add `self.OnActorEndOverlap` _output_get_4 (delegate `OnHUDTriggerExit`)))
    (:`then_5`
      ;[1 1 1] Create the levels adding them to the array
      (`KismetArrayLibrary.Array_Add` _levels (make `/Game/PAZ/Blueprint/LevelInfo` "Try Not To Miss" 99 -1 0 2))
      (`KismetArrayLibrary.Array_Add` _levels (make `/Game/PAZ/Blueprint/LevelInfo` "Level2" 50 -1 3 0 50.0))
      ;[1 1 1] Create a reference to the balloon spawner
      (bind _outactors_2 (`GameplayStatics.GetAllActorsOfClass` "/Game/PAZ/Blueprint/BP_BalloonSpawner.BP_BalloonSpawner_C"))
      (bind _output_get_5 (set `self.BalloonSpawner` (`KismetArrayLibrary.Array_Get` _outactors_2)))
      ;[1 1 1] Set up the first level
      (`/Game/PAZ/Widgets/HUD.OnBeginLevel` (`self.HUDWidgetInstance`))
      (`/Game/PAZ/Blueprint/BP_BalloonSpawner.SpawnAllObjectsForLevel` _output_get_5 (`KismetArrayLibrary.Array_Get` (`self.Levels`))))))

(event `OnHUDTriggerEnter` :!signature `self.OnActorBeginOverlap`
  (params (OtherActor :type "Actor Object Reference"))
  (bind _hudwidgetinstance (`self.HUDWidgetInstance`))
  ;[1 1 1] HUD TOGGLE
  (cast `/Game/FirstPersonBP/Blueprints/FirstPersonCharacter` OtherActor)
  (`Widget.SetVisibility` _hudwidgetinstance "Visible")
  (`self.EnableViewportForWidget` _hudwidgetinstance :!label _label))

(event `EnableViewportForWidget`
  (params (NewWidgetToActivate :type "Widget Object Reference"))
  ;[1 1 1] Set Active Screen
  (`Widget.SetVisibility` (`self.ActiveWidget`) "Hidden")
  (`Widget.SetVisibility` NewWidgetToActivate "Visible")
  (set `self.ActiveWidget` NewWidgetToActivate))

(event `OnHUDTriggerExit` :!signature `self.OnActorEndOverlap`
  (params (OtherActor :type "Actor Object Reference"))
  ;[1 1 1] HUD TOGGLE
  (cast `/Game/FirstPersonBP/Blueprints/FirstPersonCharacter` OtherActor)
  (`Widget.SetVisibility` (`self.HUDWidgetInstance`) "Hidden")
  (goto _label))

(event `InputAxis|MoveForward` :consume false :overrideparent false
  (params (AxisValue :type "Float (single-precision)"))
  (bind _activewidget (`self.ActiveWidget`))
  ;[1 1 1] Cursor Control on Title Screen
  (bind _asfirst_person_character (cast `/Game/FirstPersonBP/Blueprints/FirstPersonCharacter` (`GameplayStatics.GetPlayerCharacter` 0)))
  (bind _isplayerenabled (`/Game/FirstPersonBP/Blueprints/FirstPersonCharacter.isPlayerEnabled` _asfirst_person_character))
  (if _isplayerenabled
    _
    (elif (> AxisValue 0.25)
      (bind _astitle_screen (cast `/Game/PAZ/Widgets/TitleScreen` _activewidget))
      (`/Game/PAZ/Widgets/TitleScreen.OnArrowUp` _astitle_screen)
      (elif (< AxisValue -0.25)
        (bind _astitle_screen_2 (cast `/Game/PAZ/Widgets/TitleScreen` _activewidget))
        (`/Game/PAZ/Widgets/TitleScreen.OnArrowDown` _astitle_screen_2)))))

(event `InputAction|Select`
  (params (Key :type "Key Structure" :default "AnyKey"))
  (bind _activewidget (`self.ActiveWidget`))
  ;[1 1 1] Transition between Title and Goal Screen
  (:`Pressed`
    (bind _asfirst_person_character (cast `/Game/FirstPersonBP/Blueprints/FirstPersonCharacter` (`GameplayStatics.GetPlayerCharacter` 0)))
    (bind _isplayerenabled (`/Game/FirstPersonBP/Blueprints/FirstPersonCharacter.isPlayerEnabled` _asfirst_person_character))
    (if (not _isplayerenabled)
      (bind _astitle_screen (cast `/Game/PAZ/Widgets/TitleScreen` _activewidget)
        (:`then`
          (bind _iscursoronstart (`/Game/PAZ/Widgets/TitleScreen.GetIsActiveCursorOnStart` _astitle_screen))
          (if (not _iscursoronstart)
            (`self.EnableViewportForWidget` (`self.GoalScreenInstance`))
            (else
              (`Widget.SetVisibility` (`self.TitleScreenInstance`) "Hidden")
              (bind _asfirst_person_character_2 (cast `/Game/FirstPersonBP/Blueprints/FirstPersonCharacter` (`GameplayStatics.GetPlayerCharacter` 0)))
              (`/Game/FirstPersonBP/Blueprints/FirstPersonCharacter.EnableFPSPlayer` _asfirst_person_character_2))))
        (:`CastFailed`
          (cast `/Game/PAZ/Widgets/GoalScreen` _activewidget)
          (`self.EnableViewportForWidget` (`self.TitleScreenInstance`))
          (`GameplayStatics.PlaySound2D` "/Game/FirstPerson/Audio/FirstPersonTemplateWeaponFire02.FirstPersonTemplateWeaponFire02" 0.6))))))

(event `OnPlayerHasShot`
  ;[1 1 1] When Player Shoots
  (bind _ashud (cast `/Game/PAZ/Widgets/HUD` (`self.ActiveWidget`)))
  (`/Game/PAZ/Widgets/HUD.OnShot` _ashud "Nice Shoot!")
  (`KismetSystemLibrary.Delay` 1.5)
  (bind _levelcompleted (`self.BalloonGoalCheck`))
  (if _levelcompleted
    (`/Game/PAZ/Widgets/HUD.OnLevelCompleted` _ashud)
    (else
      (`/Game/PAZ/Widgets/HUD.OnGameOver` _ashud "Not enough Balloons"))))

(fn `BalloonGoalCheck`
  (returns (levelCompleted :type Boolean))
  (bind (_item_level_name _item_total_balloons _item_goal_balloons) (break `/Game/PAZ/Blueprint/LevelInfo` (`KismetArrayLibrary.Array_Get` (`self.Levels`) (`self.CurrentLevelIndex`))))
  ;[1 1 1] Are the remaining ballooons in level enough to have finished level
  (bind _outactors (`GameplayStatics.GetAllActorsOfClass` "/Game/PAZ/Blueprint/BP_Balloon.BP_Balloon_C"))
  (return (<= (`KismetArrayLibrary.Array_Length` _outactors) (- _item_total_balloons _item_goal_balloons))))

(fn `OnBalloonPopped`
  (`/Game/PAZ/Widgets/HUD.OnBalloonHit` (`self.HUDWidgetInstance`)))

(fn `OnLevelCompleteAnimationComplete`
  (bind _levels (`self.Levels`))
  (bind _result (`/Engine/EditorBlueprintResources/StandardMacros.IncrementInt` (`self.CurrentLevelIndex`))
    (:`  `
      (if (== _result (`KismetArrayLibrary.Array_Length` _levels))
        (`KismetSystemLibrary.PrintString` "THAT WAS LAST LEVEL SUCKER")
        (else
          (`self.SetUpNextLevel` (`KismetArrayLibrary.Array_Get` _levels _result)))))))

(fn `OnTimeEnd`
  (`/Game/PAZ/Widgets/HUD.OnGameOver` (`self.HUDWidgetInstance`) "Out of Time!"))

(fn `SetUpNextLevel`
  (params (NextLevelInfo :type "/Game/PAZ/Blueprint/LevelInfo Structure"))
  (`/Game/PAZ/Widgets/HUD.OnStartNextLevel` (`self.HUDWidgetInstance`) NextLevelInfo)
  (`/Game/PAZ/Blueprint/BP_BalloonSpawner.SpawnAllObjectsForLevel` (`self.BalloonSpawner`) NextLevelInfo))

(fn `UserConstructionScript`)