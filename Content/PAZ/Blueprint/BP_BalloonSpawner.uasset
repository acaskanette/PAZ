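; Spawner actor that fills a box-shaped area with a fixed batch of BP_Balloon actors when play begins.
; The construction script sizes the Box component's X and Z extents from the spawn area half-width and half-height variables.
; SpawnBalloons spawns each balloon at the spawner's transform, then applies a random local offset within that width and height, using a hardcoded depth range independent of the box.
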(event `self.ReceiveBeginPlay`
  (`self.SpawnBalloons` 99))

(fn `SpawnBalloons`
  (params (Amount :type Integer))
  (bind _spawn_area_half_width (`self.Spawn Area Half Width`))
  (bind _spawn_area_half_height (`self.Spawn Area Half Height`))
  ;[1 1 1] Loop through and spawn balloons at center of spawner
  (for _ (range Amount)
    (bind _returnvalue (`|SpawnActorFromClass` "/Game/PAZ/Blueprint/BP_Balloon.BP_Balloon_C" (`self.GetTransform`) "AdjustIfPossibleButAlwaysSpawn" "OverrideRootScale"))
    ;[1 1 1] Add the offset transform to the balloon's transform
    (`self.K2_AddActorLocalTransform` _returnvalue (`KismetMathLibrary.MakeTransform` (`KismetMathLibrary.MakeVector` (`KismetMathLibrary.RandomFloatInRange` (* _spawn_area_half_width -1.0) _spawn_area_half_width) (`KismetMathLibrary.RandomFloatInRange` (* 50.0 -1.0) 50.0) (`KismetMathLibrary.RandomFloatInRange` (* _spawn_area_half_height -1.0) _spawn_area_half_height)) (struct) (1.0 1.0 1.0)) false false)))

(fn `UserConstructionScript`
  (bind _box (`self.Box`))
  ;[1 1 1] Set the box extents based on blueprint parameters
  (`BoxComponent.SetBoxExtent` _box (`KismetMathLibrary.MakeVector` (`self.Spawn Area Half Width`) (.y (`BoxComponent.BoxExtent` _box)) (`self.Spawn Area Half Height`)) false))